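; Quest manager actor component that tracks in-progress and completed quests by ID for its owner in a top-down game.
; Starting or completing a quest updates those lists and tells the top-down HUD to refresh its quests.
; CanComplete reads the Quests data table: Talk quests need all related quests completed, while Objects quests check the owner's inventory component for enough of the required item, ignoring related quests.
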(event EventBeginPlay)

(event EventTick
  (params (DeltaSeconds :type Float%20%28single-precision%29)))

(fn CompleteQuest
  (params (ID :type Name))
  (Utilities|Array|RemoveItem (Variables|Default|GetInProgress) ID)
  (Utilities|Array|AddUnique (Variables|Default|GetCompleted) ID)
  (bind _asbp_top_down_hud (Utilities|Casting|CastToBP_TopDown_HUD (HUD|GetHUD (Game|GetPlayerController 0))))
  (Default|UpdateQuests _asbp_top_down_hud))

(fn StartQuest
  (params (ID :type Name))
  (if (!= ID "")
    (Utilities|Array|AddUnique (Variables|Default|GetInProgress) ID)
    (bind _asbp_top_down_hud (Utilities|Casting|CastToBP_TopDown_HUD (HUD|GetHUD (Game|GetPlayerController 0))))
    (Default|UpdateQuests _asbp_top_down_hud)))

(fn CanComplete
  (params (ID :type Name))
  (bind _returnvalue (Components|GetOwner))
  (bind _returnvalue_2 (Actor|GetComponentbyClass _returnvalue "/Game/Inventory/AC_Inventory.AC_Inventory_C"))
  (bind _returnvalue_3 (Utilities|GetDataTableRow (Variables|Default|GetQuests) ID)
    (:then
      (switch Utilities|FlowControl|Switch|SwitchonE_QuestType (.Type (Utilities|Struct|BreakF_Quest _returnvalue_3))
        (:NewEnumerator0
          ;[0.15 0.15 0.15 0.5] Si no hay tareas relacionadas, se puede completar. Si no, comprobar si las relacionadas ya están completas para poder completarla.
          (LocalVariables|SetCanComplete true)
          (bind _array_element (Utilities|Array|ForEachLoopwithBreak (.RelatedQuests (Utilities|Struct|BreakF_Quest _returnvalue_3)) :!label _label)
            (:LoopBody
              (if (not (Utilities|Array|ContainsItem (Variables|Default|GetCompleted) _array_element))
                (LocalVariables|SetCanComplete false)
                (goto _label Break)))
            (:Completed
              (return (LocalVariables|GetCanComplete)))))
        (:NewEnumerator2
          ;[0.15 0.15 0.15 0.5] Comprobar que se tiene el objeto en el inventario - Aquí también debería comprobarse si hay relacionadas y yay están completas antes de poder completarla
          (Utilities|IsValid _returnvalue_2
            (:Is%20Valid
              (if (.ReturnValue (Utilities|Map|Find (Variables|/Game/Inventory/AC_Inventory.AC_Inventory_C|GetInventory _returnvalue_2) (.ObjectName (Utilities|Struct|BreakF_Quest _returnvalue_3))))
                (return (>= (.Value (Utilities|Map|Find (Variables|/Game/Inventory/AC_Inventory.AC_Inventory_C|GetInventory _returnvalue_2) (.ObjectName (Utilities|Struct|BreakF_Quest _returnvalue_3)))) (.Value (Utilities|Struct|BreakF_Quest _returnvalue_3))))))))))
    (:RowNotFound
      (return false))))