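; BP_Potion_Health is an interactable health potion pickup that always allows interaction.
; On Interact by a BP_TopDownCharacter with a valid AC_Inventory component, it adds its ItemType row name to that inventory and destroys itself.
; It also prints the row name as debug output, and a disconnected branch holds an unused ApplyItem path that would apply the item directly.
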(event EventBeginPlay)

(event Collision|EventActorBeginOverlap
  (params (OtherActor :type Actor%20Object%20Reference)))

(event EventTick
  (params (DeltaSeconds :type Float%20%28single-precision%29)))

(event EventInteract
  (params (InteractActor :type Actor%20Object%20Reference))
  (bind _itemtype (Variables|Default|GetItemType))
  (bind _asbp_top_down_character (Utilities|Casting|CastToBP_TopDownCharacter InteractActor))
  (Utilities|IsValid (Actor|GetComponentbyClass _asbp_top_down_character "/Game/Inventory/AC_Inventory.AC_Inventory_C")
    (:Is%20Valid
      (Development|PrintString (Utilities|String|ToString(Name) (.rowname _itemtype)))
      (Default|AddtoInventory (Actor|GetComponentbyClass _asbp_top_down_character "/Game/Inventory/AC_Inventory.AC_Inventory_C") (.rowname _itemtype))
      (Actor|DestroyActor))))

(fn ConstructionScript)

(fn CanInteract
  (return true))