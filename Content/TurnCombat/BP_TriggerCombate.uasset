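; BP_TriggerCombate is a trigger that starts turn-based combat when the top-down player character overlaps its collision component.
; If the character is not already in combat, it has TurnBaseGameMode prepare the fight, passing the PosJugador world transform, the associated combatants and the flee probability.
; It then calls PrepararCombate on each associated combatant.
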(event OnComponentBeginOverlap(CollisionComponent)
  (params (OverlappedComponent :type Primitive%20Component%20Object%20Reference) (OtherActor :type Actor%20Object%20Reference) (OtherComp :type Primitive%20Component%20Object%20Reference) (OtherBodyIndex :type Integer) (bFromSweep :type Boolean) (SweepResult :type Hit%20Result%20Structure%20%28by%20ref%29))
  (bind _posjugador (Variables|Default|GetPosJugador))
  (bind _asbp_top_down_character (Utilities|Casting|CastToBP_TopDownCharacter OtherActor))
  (if (not (Variables|/Game/TopDown/Blueprints/BP_TopDownCharacter.BP_TopDownCharacter_C|GetEstaEnCombate _asbp_top_down_character))
    (bind _asturn_base_game_mode (Utilities|Casting|CastToTurnBaseGameMode (Game|GetGameMode)))
    (Default|PrepararCombate _asturn_base_game_mode (Transformation|GetWorldLocation _posjugador) (Transformation|GetWorldRotation _posjugador) (Variables|Default|GetCombatientesAsociados) (Variables|Default|GetProbabilidadHuirDeCombate))
    (for _array_element (Variables|Default|GetCombatientesAsociados)
      (Default|PrepararCombate _array_element))))

(event EventBeginPlay)

(event Collision|EventActorBeginOverlap
  (params (OtherActor :type Actor%20Object%20Reference)))

(event EventTick
  (params (DeltaSeconds :type Float%20%28single-precision%29)))

(fn ConstructionScript)