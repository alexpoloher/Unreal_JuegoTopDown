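; Double sliding door that stays locked until the top-down character overlaps it carrying a key of the matching type.
; On overlap, it looks up each player inventory item in DT_Item and compares its type to TipoLlave.
; A match removes the key, shows a HUD message and opens the door; otherwise the HUD says a key is needed.
; OpenDoor slides both leaves apart with a timeline lerp, or reverses it to close.
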(event Custom|OpenDoor
  (params (Open :type Boolean))
  (if Open
    (bind _newtrack_0 (Timeline|Timeline Play) ; Si hay que abrir, se llama al play, y si es no Open, se llama al reverse
      (:Update
        (Transformation|SetRelativeLocation (Variables|Default|GetRightDoor) (Math|Vector|Lerp(Vector) (Variables|Default|GetInitPosRightDoor) (+ (Variables|Default|GetInitPosRightDoor) "32.000000,0.000000,0.000000") _newtrack_0) false false)
        (Transformation|SetRelativeLocation (Variables|Default|GetLeftDoor) (Math|Vector|Lerp(Vector) (Variables|Default|GetInitPosLeftDoor) (+ (Variables|Default|GetInitPosLeftDoor) "-32.000000,0.000000,0.000000") _newtrack_0) false false)))
    (else
      (Timeline|Timeline Reverse))))

(event EventBeginPlay
  (Variables|Default|SetInitPosRightDoor (Variables|/Script/Engine.SceneComponent|GetRelativeLocation (Variables|Default|GetRightDoor)))
  (Variables|Default|SetInitPosLeftDoor (Variables|/Script/Engine.SceneComponent|GetRelativeLocation (Variables|Default|GetLeftDoor))))

(event Collision|EventActorBeginOverlap
  (params (OtherActor :type Actor%20Object%20Reference))
  (bind _returnvalue (Game|GetPlayerCharacter 0))
  (bind _returnvalue_2 (Game|GetPlayerController 0))
  (bind _returnvalue_3 (Actor|GetComponentbyClass _returnvalue "/Game/Inventory/AC_Inventory.AC_Inventory_C"))
  (bind _returnvalue_4 (HUD|GetHUD _returnvalue_2))
  (if (not (Variables|Default|GetPuertaAbierta))
    (Utilities|Casting|CastToBP_TopDownCharacter OtherActor)
    (Utilities|IsValid _returnvalue_3
      (:Is%20Valid
        (bind _keys (Utilities|Map|Keys (Variables|/Game/Inventory/AC_Inventory.AC_Inventory_C|GetInventory _returnvalue_3)))
        (for _array_element _keys
          (bind _returnvalue_5 (Utilities|GetDataTableRow "/Game/Inventory/DT_Item.DT_Item" _array_element)
            (:then
              (if (Utilities|Enum|Equal(Enum) (.type _returnvalue_5) (Variables|Default|GetTipoLlave))
                (Variables|Default|SetTieneLlave true)
                (Variables|Default|SetPuertaAbierta true)
                (bind _asbp_top_down_hud (Utilities|Casting|CastToBP_TopDown_HUD _returnvalue_4))
                (Default|MostrarMensaje _asbp_top_down_hud "Se ha usado la llave para abrir")
                (CallFunction|OpenDoor true)
                (bind _asbp_top_down_character (Utilities|Casting|CastToBP_TopDownCharacter (Game|Player|GetPlayerPawn 0)))
                (Default|RemovefromInventory (Variables|/Game/TopDown/Blueprints/BP_TopDownCharacter.BP_TopDownCharacter_C|GetAC_Inventory _asbp_top_down_character) (.name _returnvalue_5))))))
        (if (not (Variables|Default|GetTieneLlave))
          (bind _asbp_top_down_hud_2 (Utilities|Casting|CastToBP_TopDown_HUD _returnvalue_4))
          (Default|MostrarMensaje _asbp_top_down_hud_2 "Necesitas una llave para abrir la puerta"))))))

(event EventTick
  (params (DeltaSeconds :type Float%20%28single-precision%29)))

(fn ConstructionScript)