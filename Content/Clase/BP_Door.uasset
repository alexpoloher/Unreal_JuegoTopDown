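; BP_Door is a double sliding door whose two panels move apart and back together.
; BeginPlay caches each panel's relative location as the closed position.
; Open forwards its boolean to OpenDoor, which plays a timeline to open or reverses it to close.
; The timeline track lerps both panels along opposite relative X offsets, without sweep.
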(event Custom|OpenDoor
  (params (Open :type Boolean))
  (if Open
    (bind _newtrack_0 (Timeline|Timeline Play) ; Si hay que abrir, se llama al play, y si es no Open, se llama al reverse
      (:Update
        (Transformation|SetRelativeLocation (Variables|Default|GetRightDoor) (Math|Vector|Lerp(Vector) (Variables|Default|GetInitPosRightDoor) (+ (Variables|Default|GetInitPosRightDoor) "144.000000,0.000000,0.000000") _newtrack_0) false false)
        (Transformation|SetRelativeLocation (Variables|Default|GetLeftDoor) (Math|Vector|Lerp(Vector) (Variables|Default|GetInitPosLeftDoor) (+ (Variables|Default|GetInitPosLeftDoor) "-144.000000,0.000000,0.000000") _newtrack_0) false false)))
    (else
      (Timeline|Timeline Reverse))))

(event EventBeginPlay
  (Variables|Default|SetInitPosRightDoor (Variables|/Script/Engine.SceneComponent|GetRelativeLocation (Variables|Default|GetRightDoor)))
  (Variables|Default|SetInitPosLeftDoor (Variables|/Script/Engine.SceneComponent|GetRelativeLocation (Variables|Default|GetLeftDoor))))

(event Collision|EventActorBeginOverlap
  (params (OtherActor :type Actor%20Object%20Reference)))

(event EventTick
  (params (DeltaSeconds :type Float%20%28single-precision%29)))

(event EventOpen
  (params (Open :type Boolean))
  (CallFunction|OpenDoor Open))

(fn ConstructionScript)