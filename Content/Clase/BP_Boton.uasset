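; BP_Boton is a push button that the top-down character toggles with E while standing inside its box.
; Box overlaps enable or disable input, and each press flips Activado and swaps the blue pressed/unpressed material.
; If Door is valid and implements BP_OpenDoor, the press calls CallDoorToOpen, which only calls CallButtonChangeState.
; Direct OpenMessage calls to the door, including an open-on-overlap variant, are left unconnected.
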(event OnComponentBeginOverlap(Box)
  (params (OverlappedComponent :type Primitive%20Component%20Object%20Reference) (OtherActor :type Actor%20Object%20Reference) (OtherComp :type Primitive%20Component%20Object%20Reference) (OtherBodyIndex :type Integer) (bFromSweep :type Boolean) (SweepResult :type Hit%20Result%20Structure%20%28by%20ref%29))
  (Utilities|Casting|CastToBP_TopDownCharacter OtherActor)
  (Variables|Default|SetPlayerIsInside true)
  (Input|EnableInput (Game|GetPlayerController 0)))

(event OnComponentEndOverlap(Box)
  (params (OverlappedComponent :type Primitive%20Component%20Object%20Reference) (OtherActor :type Actor%20Object%20Reference) (OtherComp :type Primitive%20Component%20Object%20Reference) (OtherBodyIndex :type Integer))
  (Utilities|Casting|CastToBP_TopDownCharacter OtherActor)
  (Variables|Default|SetPlayerIsInside false)
  (Input|DisableInput (Game|GetPlayerController 0)))

(event Custom|CallDoorToOpen
  (params (Open :type Boolean))
  (Default|CallButtonChangeState))

(event EventBeginPlay)

(event Collision|EventActorBeginOverlap
  (params (OtherActor :type Actor%20Object%20Reference)))

(event EventTick
  (params (DeltaSeconds :type Float%20%28single-precision%29)))

(event Input|KeyboardEvents|E
  (params (Key :type Key%20Structure :default "None"))
  (bind _door (Variables|Default|GetDoor))
  (bind _staticmesh (Variables|Default|GetStaticMesh))
  (:Pressed
    (if (Variables|Default|GetPlayerIsInside)
      (bind _output_get (Variables|Default|SetActivado (not (Variables|Default|GetActivado))))
      (if _output_get
        (Rendering|Material|SetMaterial _staticmesh 0 "/Game/Clase/M_BotonAzulPulsado.M_BotonAzulPulsado")
        (else
          (Rendering|Material|SetMaterial _staticmesh 0 "/Game/Clase/M_BotonAzulNoPulsado.M_BotonAzulNoPulsado")))
      (Utilities|IsValid _door
        (:Is%20Valid
          (if (Utilities|DoesObjectImplementInterface _door "/Game/Clase/BP_OpenDoor.BP_OpenDoor_C")
            (CallFunction|CallDoortoOpen false)))))))

(fn ConstructionScript)