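; Base enemy for turn-based combat that attacks the player, takes damage and reports turn ends and death to TurnBaseGameMode.
; Each turn resolves burn or sleep, picks a weighted-random DataTable attack, rolls accuracy, then walks up, plays its montage and returns.
; An anim notify delivers hits with crit and status rolls; incoming damage scales by elemental affinity and attack/defense ratio.
; Death hides rather than destroys the actor, so fleeing can restore it.
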(event Custom|LlamarGolpearObjetivo
  ;[0.15 0.15 0.15 0.5] Anim notify de EnemyAttack, al golpear al jugador
  (CallFunction|GolpearObjetivo))

(event Custom|PerformAttack
  ;[0.15 0.15 0.15 0.5] Realizar el ataque
  (Animation|Montage|PlayMontage (Variables|Character|GetMesh) (.Value (Utilities|Map|Find (Variables|Ataques|GetIdsAtaquesYMontagesDisponibles) (Variables|Combate|GetIdSiguienteAtaque)))
    (:OnCompleted
      _)
    (:OnInterrupted
      _))
  (CallFunction|VolverAPosInicial))

(event Custom|AcercarseAlObjetivo
  (params (Destino :type Vector))
  ;[0.15 0.15 0.15 0.5] Acercarse al jugador antes de realizar el ataque
  (AI|AIMoveTo (Class|PawnMovementComponent|GetPawnOwner (Variables|Character|GetCharacterMovement)) Destino 0 5e+01 false
    (:OnSuccess
      (CallFunction|PerformAttack))))

(event Custom|PrepararCombate
  ;[0.15 0.15 0.15 0.5] Al entrar en combate, se muestra la barra de salud
  (Variables|Combate|SetEstaEnCombate true)
  (Development|SetHiddeninGame (Variables|Default|GetBarraVida) false false)
  (bind _output_get (Variables|Stats|SetVida (Variables|Stats|GetVidaMaxima)))
  (CallFunction|ModificarBarraDeVida _output_get))

(event Custom|OcultarDeEscena
  ;[0.15 0.15 0.15 0.5] Ocultar el enemigo al ser derrotado. También se elimina del array de combatientes desde el gestor del combate por turnos
  (Utilities|FlowControl|Delay 1.0)
  (Rendering|SetActorHiddenInGame self true)
  (bind _asbp_top_down_character (Utilities|Casting|CastToBP_TopDownCharacter (Game|GetPlayerCharacter 0)))
  (Default|UpdateKillProgress (Variables|/Game/TopDown/Blueprints/BP_TopDownCharacter.BP_TopDownCharacter_C|GetAC_QuestManager _asbp_top_down_character)))

(event Custom|VolverAPosInicial
  ;[0.15 0.15 0.15 0.5] Tras golpear, se vuelve hacia la posición en la que estaba
  (AI|AIMoveTo (Class|PawnMovementComponent|GetPawnOwner (Variables|Character|GetCharacterMovement)) (Variables|Movimiento|GetPosInicial) 0 5.0 false
    (:OnSuccess
      (bind _newtrack_0 (Timeline|TimelineRotarEnemigo PlayFromStart)
        (:Update
          (Transformation|SetActorRotation (Math|Rotator|Lerp(Rotator) (Variables|Movimiento|GetRotacionActual) (Variables|Movimiento|GetRotacionInicial) _newtrack_0 true)))
        (:Finished
          (bind _asturn_base_game_mode (Utilities|Casting|CastToTurnBaseGameMode (Game|GetGameMode) :!label _label))
          (Variables|Combate|SetHaAtacadoEstaRonda true)
          (Default|EndTurn _asturn_base_game_mode self))))
    (:OnFail
      (Transformation|SetActorLocationAndRotation (Variables|Movimiento|GetPosInicial) (Variables|Movimiento|GetRotacionInicial) false true)
      (goto _label))))

(event EventBeginPlay
  ;[0.15 0.15 0.15 0.5] Setup
  (bind _asbp_barra_vida_enemigo (Utilities|Casting|CastToBP_BarraVidaEnemigo (UserInterface|GetWidget (Variables|Default|GetBarraVida))))
  (Variables|Combate|SetBarraDeVidaRef _asbp_barra_vida_enemigo)
  (bind _asturn_base_game_mode (Utilities|Casting|CastToTurnBaseGameMode (Game|GetGameMode)))
  (Variables|Default|SetGameMode _asturn_base_game_mode)
  (CallFunction|ObtenerAtaques) ; Recoge qué 4 ataques tiene (o menos)
  (bind _asbp_top_down_character (Utilities|Casting|CastToBP_TopDownCharacter (Game|GetPlayerCharacter 0)))
  (Variables|Default|SetPlayer _asbp_top_down_character)
  (Variables|Stats|SetVida (Variables|Stats|GetVidaMaxima)))

(event Collision|EventActorBeginOverlap
  (params (OtherActor :type Actor%20Object%20Reference))
  ;[0.15 0.15 0.15 0.5] Setup
)

(event EventResetearStats
  ;[0.15 0.15 0.15 0.5] Resetear stats a los valores base
  (Variables|Stats|SetStatAtaque (Variables|Stats|GetStatAtaqueOriginal))
  (Variables|Stats|SetStatDefensa (Variables|Stats|GetStatDefensaOriginal))
  (Variables|Stats|SetVida (Variables|Stats|GetVidaMaxima))
  (Variables|Combate|SetEstadoAplicado "NewEnumerator1")
  (Variables|Combate|SetTurnosResantesDeEstado 0))

(event EventHuyeDelCombate
  ;[0.15 0.15 0.15 0.5] CuandoElJugadorHuyeDelCombate
  (Variables|Combate|SetMuerto false)
  (Variables|Combate|SetEstaEnCombate false)
  (Development|SetHiddeninGame (Variables|Default|GetBarraVida) true true)
  (CallFunction|ResetearStats)
  (Utilities|FlowControl|Delay 1.0)
  (Rendering|SetActorHiddenInGame self false))

(event EventTick
  (params (DeltaSeconds :type Float%20%28single-precision%29))
  (bind _barravida (Variables|Default|GetBarraVida))
  ;[0.15 0.15 0.15 0.5] Gestión de barra de vida de enemigos - Siempre apuntan a cámara
  (if (Variables|Combate|GetEstaEnCombate)
    (Transformation|SetWorldRotation _barravida (Math|Rotator|FindLookatRotation (Transformation|GetWorldLocation _barravida) (Transformation|GetWorldLocation (Variables|/Script/Engine.PlayerCameraManager|GetTransformComponent (Game|GetPlayerCameraManager 0)))) false false)))

(event EventStartTurn
  ;[0.15 0.15 0.15 0.5] Inicio del turno del enemigo
  (if (Utilities|Enum|Equal(Enum) (Variables|Combate|GetEstadoAplicado) "NewEnumerator1")
    (CallFunction|SeleccionarAtaque :!label _label)
    (bind _puedegolpear (CallFunction|ComprobarSiGolpea))
    (if _puedegolpear
      (CallFunction|CalcularPosObjetivo (Variables|Default|GetPlayer))
      (else
        (CallFunction|FallaElAtaque)))
    (else
      (bind (_hamuerto _golpeaesteturno _sufredanio) (CallFunction|AplicarEfectoDeEstado))
      (CallFunction|DescontarTurnoDeEstado)
      (if (and (== _hamuerto false) (== _golpeaesteturno true)) ; Si no ha muerto y puede golpear, golpea
        (if _sufredanio
          (Animation|Montage|PlayMontage (Variables|Character|GetMesh) (Variables|Combate|GetMontageHit)
            (:OnCompleted
              (goto _label)))
          (else
            (goto _label)))
        (elif _hamuerto
          (CallFunction|Morir)
          (Default|EndTurn (Variables|Default|GetGameMode) self)
          (else
            (Variables|Combate|SetHaAtacadoEstaRonda true)
            (Default|EndTurn (Variables|Default|GetGameMode) self)))))))

(event EventInteract
  (params (InteractActor :type Actor%20Object%20Reference)))

(event EventRecibirEfecto
  (params (TipoEfecto :type E_EfectosPosibles%20Enum :default "NewEnumerator1") (TurnosAAplicar :type Integer))
  ;[0.15 0.15 0.15 0.5] Aplicar un efecto secundario al enemigo
  (switch Utilities|FlowControl|Switch|SwitchonE_EfectosPosibles TipoEfecto
    (:NewEnumerator0
      (CallFunction|AplicarQuemadura TurnosAAplicar) ; Se separan porque podría añadirse que cada uno hicese además cosas distintas
    )
    (:NewEnumerator2
      (CallFunction|AplicarSueño TurnosAAplicar))))

(event EventRecibirGolpe
  (params (Damage :type Integer) (AplicaEfectoSecundario :type Boolean) (TipoEfectoSecundario :type E_EfectosPosibles%20Enum :default "NewEnumerator1") (CantidadEfectoSecundario :type Integer) (ElementoDelAtaque :type E_Elementos%20Enum :default "NewEnumerator0") (StatAtaque :type Integer))
  ;[0.15 0.15 0.15 0.5] Recibir daño
  (bind _damageaplicar (CallFunction|CalcularDanioFinal Damage ElementoDelAtaque StatAtaque))
  (CallFunction|ModificarBarraDeVida (- (Variables|Stats|GetVida) _damageaplicar))
  (if (<= (- (Variables|Stats|GetVida) _damageaplicar) 0)
    (Variables|Stats|SetVida 0)
    (CallFunction|Morir)
    (else
      (Variables|Stats|SetVida (- (Variables|Stats|GetVida) _damageaplicar))
      (Animation|PlayAnimMontage (Variables|Combate|GetMontageHit) 1.0 "None")
      (if AplicaEfectoSecundario
        (CallFunction|RecibirEfecto TipoEfectoSecundario CantidadEfectoSecundario)))))

(event EventFallaElAtaque
  ;[0.15 0.15 0.15 0.5] Si se falla el ataque
  (Animation|Montage|PlayMontage (Variables|Character|GetMesh) (Variables|Combate|GetMontageFallaAtaque)
    (:OnCompleted
      (Variables|Combate|SetHaAtacadoEstaRonda true)
      (Utilities|FlowControl|Delay 0.75)
      (Default|EndTurn (Variables|Default|GetGameMode) self))))

(event EventComenzarNuevaRonda
  ;[0.15 0.15 0.15 0.5] Gestiones de ronda
  (Variables|Combate|SetHaAtacadoEstaRonda false))

(event EventSetVelocidadEnRonda
  (params (VelocidadEnRonda :type Integer))
  ;[0.15 0.15 0.15 0.5] Gestiones de ronda
  (Variables|Combate|SetVelocidadEnRonda VelocidadEnRonda))

(fn ConstructionScript)

(fn SeleccionarAtaque
  (Utilities|FlowControl|Sequence
    (:then_1
      ;[0.15 0.15 0.15 0.5] Se genera un random, y el escogido será el primero cuyo peso sea igual o mayor que el generado
      (LocalVariables|SetPesoAcumulado 0)
      (LocalVariables|SetValorPesoAtaqueSeleccionado (Math|Random|RandomInteger (Variables|Ataques|GetPesoTotalAtaques)))
      (bind _keys (Utilities|Map|Keys (Variables|Ataques|GetMapaAtaquesPoseidos)))
      (for _array_element _keys
        (LocalVariables|SetPesoAcumulado (+ (LocalVariables|GetPesoAcumulado) (.PesoEleccion (Utilities|Struct|BreakS_EnemiesAttacks (.Value (Utilities|Map|Find (Variables|Ataques|GetMapaAtaquesPoseidos) _array_element))))))
        (if (>= (LocalVariables|GetPesoAcumulado) (LocalVariables|GetValorPesoAtaqueSeleccionado))
          (Variables|Combate|SetIdSiguienteAtaque _array_element)
          (return _array_element))))))

(fn ObtenerAtaques
  (Variables|Ataques|SetPesoTotalAtaques 0)
  (bind _keys (Utilities|Map|Keys (Variables|Ataques|GetIdsAtaquesYMontagesDisponibles)))
  (for _array_element _keys
    (bind _returnvalue (Utilities|GetDataTableRow (Variables|Ataques|GetDataTableAtaques) _array_element)
      (:then
        (Utilities|Map|Add (Variables|Ataques|GetMapaAtaquesPoseidos) _array_element _returnvalue)
        (Variables|Ataques|SetPesoTotalAtaques (+ (Variables|Ataques|GetPesoTotalAtaques) (.PesoEleccion (Utilities|Struct|BreakS_EnemiesAttacks _returnvalue))))))))

(fn GolpearObjetivo
  (bind _player (Variables|Default|GetPlayer))
  (bind _idsiguienteataque (Variables|Combate|GetIdSiguienteAtaque))
  (bind _mapaataquesposeidos (Variables|Ataques|GetMapaAtaquesPoseidos))
  (bind _value (Utilities|Map|Find _mapaataquesposeidos _idsiguienteataque))
  (bind (_nombre _damage _costepm _description _precision _pesoeleccion _probabilidadefectosecundario _efectoqueaplica _cantidadefecto _elemento) (Utilities|Struct|BreakS_EnemiesAttacks _value))
  (if (Utilities|DoesObjectImplementInterface _player "/Game/TurnCombat/I_CombatPlayer.I_CombatPlayer_C")
    (bind _escritico (CallFunction|ComprobarSiEsCritico))
    (if _escritico
      (LocalVariables|SetDamageAAplicar (* _damage (Variables|Stats|GetDanioCritico)))
      (else
        (LocalVariables|SetDamageAAplicar _damage)))
    (switch Utilities|FlowControl|Switch|SwitchonE_EfectosPosibles _efectoqueaplica
      (:NewEnumerator1
        _)
      (:NewEnumerator0
        (bind _aplicaefecto (CallFunction|ComprobarSiAplicaEfectoSecundario _probabilidadefectosecundario :!label _label))
        (if _aplicaefecto
          (LocalVariables|SetAplicaEfecto true)
          (LocalVariables|SetEfectoQueAplica _efectoqueaplica)
          (LocalVariables|SetCantidadDeTurnos _cantidadefecto)
          (else
            (LocalVariables|SetAplicaEfecto false))))
      (:NewEnumerator2
        (goto _label)))
    (Default|RecibirGolpe _player (LocalVariables|GetDamageAAplicar) (LocalVariables|GetAplicaEfecto) (LocalVariables|GetEfectoQueAplica) (LocalVariables|GetCantidadDeTurnos) _elemento (Variables|Stats|GetStatAtaque))))

(fn CalcularPosObjetivo
  (params (Objetivo :type Actor%20Object%20Reference))
  (bind _returnvalue (Transformation|GetActorLocation Objetivo))
  (Variables|Movimiento|SetPosInicial (Transformation|GetActorLocation))
  (Variables|Movimiento|SetRotacionInicial (Transformation|GetActorRotation))
  (bind _output_get (LocalVariables|SetPosDelObjetivo (+ (* (Math|Vector|Normalize (- (Transformation|GetActorLocation) _returnvalue)) (Variables|Movimiento|GetStopDistance)) _returnvalue)))
  (CallFunction|AcercarseAlObjetivo _output_get))

(fn AplicarQuemadura
  (params (NumTurnosAAplicar :type Integer))
  (if (or (Utilities|Enum|Equal(Enum) (Variables|Combate|GetEstadoAplicado) "NewEnumerator1") (Utilities|Enum|Equal(Enum) (Variables|Combate|GetEstadoAplicado) "NewEnumerator0")) ; Solo se aplica quemadura si no tiene estado o ya está quemado
    (if (< (Variables|Combate|GetTurnosResantesDeEstado) NumTurnosAAplicar)
      (Variables|Combate|SetEstadoAplicado "NewEnumerator0")
      (Variables|Combate|SetTurnosResantesDeEstado NumTurnosAAplicar)
      (Default|MostrarIconoDeEstado (Variables|Combate|GetBarraDeVidaRef) "NewEnumerator0"))))

(fn AplicarSueño
  (params (NumTurnosAAplicar :type Integer))
  (if (or (Utilities|Enum|Equal(Enum) (Variables|Combate|GetEstadoAplicado) "NewEnumerator1") (Utilities|Enum|Equal(Enum) (Variables|Combate|GetEstadoAplicado) "NewEnumerator2")) ; Solo se aplica sueño si no tiene estado o ya está dormido
    (if (< (Variables|Combate|GetTurnosResantesDeEstado) NumTurnosAAplicar)
      (Variables|Combate|SetEstadoAplicado "NewEnumerator2")
      (Variables|Combate|SetTurnosResantesDeEstado NumTurnosAAplicar)
      (Default|MostrarIconoDeEstado (Variables|Combate|GetBarraDeVidaRef) "NewEnumerator2"))))

(fn AplicarEfectoDeEstado
  (switch Utilities|FlowControl|Switch|SwitchonE_EfectosPosibles (Variables|Combate|GetEstadoAplicado)
    (:NewEnumerator0
      (LocalVariables|SetHaSufridoDanio true)
      (bind _output_get (Variables|Stats|SetVida (- (Variables|Stats|GetVida) (/ (* (Variables|Stats|GetVidaMaxima) 10) 100))))
      (CallFunction|ModificarBarraDeVida _output_get)
      (if (<= _output_get 0)
        (LocalVariables|SetMuere true)
        (Variables|Stats|SetVida 0)
        (else
          (LocalVariables|SetMuere false))))
    (:NewEnumerator2
      (LocalVariables|SetPuedeGolpearEsteTurno false)))
  (return (LocalVariables|GetMuere) (LocalVariables|GetPuedeGolpearEsteTurno) (LocalVariables|GetHaSufridoDanio)))

(fn DescontarTurnoDeEstado
  (bind _result (Math|Integer|DecrementInt (Variables|Combate|GetTurnosResantesDeEstado))
    (:%20%20
      (if (== _result 0)
        (Variables|Combate|SetEstadoAplicado "NewEnumerator1")
        (Default|OcultarIconoDeEstado (Variables|Combate|GetBarraDeVidaRef))))))

(fn ModificarBarraDeVida
  (params (VidaActual :type Integer))
  (if (< VidaActual 0)
    (LocalVariables|SetLaVidaActual 0.0)
    (else
      (LocalVariables|SetLaVidaActual (Math|Conversions|ToFloat(Integer) VidaActual))))
  (Variables|/Script/UMG.ProgressBar|SetPercent (Variables|/Game/UI/CombateTurnos/BP_BarraVidaEnemigo.BP_BarraVidaEnemigo_C|GetBarraVida (Variables|Combate|GetBarraDeVidaRef)) (/ (LocalVariables|GetLaVidaActual) (Variables|Stats|GetVidaMaxima))))

(fn Morir
  ;[0.15 0.15 0.15 0.5] Al morir se reitra de los combatientes
  (Variables|Combate|SetMuerto true)
  (bind _asturn_base_game_mode (Utilities|Casting|CastToTurnBaseGameMode (Game|GetGameMode)))
  (Default|UnregisterCombatPlayer _asturn_base_game_mode self)
  (Development|SetHiddeninGame (Variables|Default|GetBarraVida) true false)
  (CallFunction|OcultarDeEscena))

(fn ComprobarSiGolpea
  (if (< (Math|Random|RandomInteger 100) (.Precision (Utilities|Struct|BreakS_EnemiesAttacks (.Value (Utilities|Map|Find (Variables|Ataques|GetMapaAtaquesPoseidos) (Variables|Combate|GetIdSiguienteAtaque))))))
    (LocalVariables|SetHaAcertado true)
    (else
      (LocalVariables|SetHaAcertado false)))
  (return (LocalVariables|GetHaAcertado)))

(fn CalcularDanioFinal
  (params (DamageAtaque :type Integer) (ElementoAtaque :type E_Elementos%20Enum :default "NewEnumerator0") (StatAtaque :type Integer))
  (LocalVariables|SetDamageFinal DamageAtaque)
  (if (or (Utilities|Enum|Equal(Enum) ElementoAtaque "NewEnumerator0") (Utilities|Enum|Equal(Enum) (Variables|Stats|GetElemento) "NewEnumerator0")) ; Si el ataque no tiene elemento, o yo tampoco, me pega normal
    (bind _damagefinal (CallFunction|CalcularModificadorAtaqueDefensa (LocalVariables|GetDamageFinal) StatAtaque))
    (return _damagefinal)
    (else
      (bind _outrownames (DataTable|GetDataTableRowNames (Variables|Default|GetDataTableElementos)))
      (for _array_element _outrownames
        (bind _returnvalue (Utilities|GetDataTableRow (Variables|Default|GetDataTableElementos) _array_element)
          (:then
            (if (Utilities|Enum|Equal(Enum) (Variables|Stats|GetElemento) (.Elemento (Utilities|Struct|BreakS_InfoElementos _returnvalue))) ; Busco mi elemento en la tabla de elementos
              (if (Utilities|Enum|Equal(Enum) (.DebilAnte (Utilities|Struct|BreakS_InfoElementos _returnvalue)) ElementoAtaque)
                ;[0.15 0.15 0.15 0.5] Si es mi debilidad, me golpea x2
                (LocalVariables|SetDamageFinal (* (LocalVariables|GetDamageFinal) 2))
                (elif (Utilities|Enum|Equal(Enum) (.FuerteContra (Utilities|Struct|BreakS_InfoElementos _returnvalue)) ElementoAtaque)
                  ;[0.15 0.15 0.15 0.5] Si es el elemento que resisto, me golpea la mitad
                  (if (< (/ (LocalVariables|GetDamageFinal) 2) 1)
                    (LocalVariables|SetDamageFinal 1) ; Mínimo hace 1 de daño
                    (else
                      (LocalVariables|SetDamageFinal (/ (LocalVariables|GetDamageFinal) 2))))))
              (bind _damagefinal_2 (CallFunction|CalcularModificadorAtaqueDefensa (LocalVariables|GetDamageFinal) StatAtaque))
              (return _damagefinal_2))))))))

(fn CalcularModificadorAtaqueDefensa
  (params (Damage :type Integer) (StatAtaque :type Integer))
  (bind _statdefensa (Variables|Stats|GetStatDefensa))
  (bind _returnvalue (+ StatAtaque _statdefensa))
  (bind _returnvalue_2 (Math|Conversions|ToFloat(Integer) _returnvalue))
  (bind _returnvalue_3 (/ StatAtaque _returnvalue_2))
  (bind _returnvalue_4 (* Damage _returnvalue_3))
  (bind _returnvalue_5 (Math|Float|Truncate _returnvalue_4))
  ;[0.15 0.15 0.15 0.5] Para tener en cuenta ataque y defensa, se aplica una fórmula para obtener una cantidad que multiplicará el ataque. Si Tnego el doble de ataque que el enemigo defensa, le haré todo el daño. De llo contrario, de forma gradual,. ese porcentaje va decrementando
  (if (< _returnvalue_5 1)
    (LocalVariables|SetDamageFinalCalculado 1)
    (else
      (LocalVariables|SetDamageFinalCalculado _returnvalue_5)))
  (return (LocalVariables|GetDamageFinalCalculado)))

(fn CanInteract
  (return true))

(fn ComprobarSiAplicaEfectoSecundario
  (params (ProbabilidadDeAplicarEfecto :type Float%20%28double-precision%29))
  (return (> ProbabilidadDeAplicarEfecto (Math|Random|RandomFloatinRange 0.0 1e+02))))

(fn ComprobarSiEsCritico
  (if (< (Math|Random|RandomFloatinRange 0.0 99.0) (Variables|Stats|GetProbCritico))
    (LocalVariables|SetGolpeCritico true)
    (else
      (LocalVariables|SetGolpeCritico false)))
  (return (LocalVariables|GetGolpeCritico)))

(fn GetVelocidadEnRonda
  (return (Variables|Combate|GetVelocidadEnRonda)))

(fn ObtenerHaAtacadoEstaRonda
  (return (Variables|Combate|GetHaAtacadoEstaRonda)))

(fn ObtenerVelocidad
  (return (Variables|Stats|GetAttackSpeed)))