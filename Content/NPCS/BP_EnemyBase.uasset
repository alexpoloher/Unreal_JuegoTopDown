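; Base enemy Blueprint for turn-based combat, exposing speed and has-attacked state per round, plus an interact stub.
; Its turn is a placeholder that prints, waits, marks itself as attacked and calls EndTurn on TurnBaseGameMode.
; Hits reduce Vida and play a montage, or at zero unregister it from combat and destroy it.
; BeginPlay only casts the game mode, as the combat registration call is disconnected.
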(event EventBeginPlay
  (bind _asturn_base_game_mode (Utilities|Casting|CastToTurnBaseGameMode (Game|GetGameMode))))

(event Collision|EventActorBeginOverlap
  (params (OtherActor :type Actor%20Object%20Reference)))

(event EventTick
  (params (DeltaSeconds :type Float%20%28single-precision%29)))

(event EventStartTurn
  (Development|PrintString (Utilities|String|Append "Turn of" (Utilities|GetDisplayName self)))
  (Utilities|FlowControl|Delay 2.5)
  (bind _asturn_base_game_mode (Utilities|Casting|CastToTurnBaseGameMode (Game|GetGameMode)))
  (Variables|Default|SetHaAtacadoEstaRonda true)
  (Default|EndTurn _asturn_base_game_mode self))

(event EventInteract
  (params (InteractActor :type Actor%20Object%20Reference))
  (Development|PrintString "Interacting with NPC"))

(event EventRecibirGolpe
  (params (Damage :type Integer))
  (if (<= (- (Variables|Default|GetVida) Damage) 0)
    (Variables|Default|SetVida 0)
    ;[0.15 0.15 0.15 0.5] Al morir, se le retira de los ocmbatientes
    (bind _asturn_base_game_mode (Utilities|Casting|CastToTurnBaseGameMode (Game|GetGameMode)))
    (Default|UnregisterCombatPlayer _asturn_base_game_mode self)
    (Actor|DestroyActor)
    (else
      (Variables|Default|SetVida (- (Variables|Default|GetVida) Damage))
      (Animation|PlayAnimMontage "/Game/NPCS/MontajesCombateNpcs/Montage_SimpleHit.Montage_SimpleHit" 1.0 "None"))))

(event EventComenzarNuevaRonda
  (Variables|Default|SetHaAtacadoEstaRonda false))

(event EventSetVelocidadEnRonda
  (params (VelocidadEnRonda :type Integer))
  (Variables|Default|SetVelocidadEnRonda VelocidadEnRonda))

(fn ConstructionScript)

(fn NewFunction)

(fn NewFunction0)

(fn CanInteract
  (return true))

(fn GetVelocidadEnRonda
  (return (Variables|Default|GetVelocidadEnRonda)))

(fn ObtenerHaAtacadoEstaRonda
  (return (Variables|Default|GetHaAtacadoEstaRonda)))

(fn ObtenerVelocidad
  (return (Variables|Default|GetAttackSpeed)))