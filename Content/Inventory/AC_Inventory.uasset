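; Actor component that stores an inventory as a map from item IDs to stack counts.
; AddToInventory increments the count of an existing entry or creates one at a count of one.
; RemoveFromInventory decrements an existing entry and deletes it once the count reaches zero or below.
; The event graph holds no logic, so changes happen only through these two functions.
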(event EventBeginPlay)

(event EventTick
  (params (DeltaSeconds :type Float%20%28single-precision%29)))

(fn AddtoInventory
  (params (ItemId :type Name))
  (bind _inventory (Variables|Default|GetInventory))
  (bind (_value _returnvalue) (Utilities|Map|Find _inventory ItemId))
  (if _returnvalue
    (Utilities|Map|Add _inventory ItemId (+ _value 1))
    (else
      (Utilities|Map|Add _inventory ItemId 1))))

(fn RemovefromInventory
  (params (ItemId :type Name))
  (bind _inventory (Variables|Default|GetInventory))
  (bind (_value _returnvalue) (Utilities|Map|Find _inventory ItemId))
  (if _returnvalue
    (bind _result (Math|Integer|DecrementInt _value)
      (:%20%20
        (if (<= _result 0)
          (Utilities|Map|Remove _inventory ItemId)
          (else
            (Utilities|Map|Add _inventory ItemId _result)))))))